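; Spear trap that thrusts out while the player is in range and deals heavy damage on contact.
; StartRange overlaps with BP_Player set and clear the StartArrow flag.
; Tick plays the TimeArrow timeline while the flag is set, moving ArrowMesh along local Z; once cleared, the timeline keeps playing until Z reaches zero, then stops.
; ArrowBox applies damage to any BP_Player that overlaps it.
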(event `self.ArrowBox.OnComponentBeginOverlap`
  (params (OverlappedComponent :type "PrimitiveComponent Object Reference") (OtherActor :type "Actor Object Reference") (OtherComp :type "PrimitiveComponent Object Reference") (OtherBodyIndex :type Integer) (bFromSweep :type Boolean) (SweepResult :type "HitResult Structure (by ref)"))
  ;[1 1 1] 当たり判定
  (bind _asbp_player (cast `/Game/Ookouchi/Character/BP/BP_Player` OtherActor))
  (`GameplayStatics.ApplyDamage` _asbp_player 100.0))

(event `self.ReceiveTick`
  (params (DeltaSeconds :type "Float (single-precision)"))
  ;[1 1 1] 出し入れ処理
  (if (`self.StartArrow`)
    (bind (_direction _arrowz) (`Timeline|TimeArrow` :!label _label)
      (:`Update`
        (`SceneComponent.K2_SetRelativeLocation` (`self.ArrowMesh`) (`KismetMathLibrary.MakeVector` 0.0 0.0 _arrowz) false false)))
    (elif (== _arrowz 0.0)
      (goto _label :!via `Stop`)
      (else
        (goto _label)))))

(event `self.StartRange.OnComponentBeginOverlap`
  (params (OverlappedComponent :type "PrimitiveComponent Object Reference") (OtherActor :type "Actor Object Reference") (OtherComp :type "PrimitiveComponent Object Reference") (OtherBodyIndex :type Integer) (bFromSweep :type Boolean) (SweepResult :type "HitResult Structure (by ref)"))
  ;[1 1 1] 起動処理
  (cast `/Game/Ookouchi/Character/BP/BP_Player` OtherActor)
  (set `self.StartArrow` true) ; Trueにする
  (if (`self.StartArrow`) :!label _label_2
    _))

(event `self.StartRange.OnComponentEndOverlap`
  (params (OverlappedComponent :type "PrimitiveComponent Object Reference") (OtherActor :type "Actor Object Reference") (OtherComp :type "PrimitiveComponent Object Reference") (OtherBodyIndex :type Integer))
  ;[1 1 1] 起動処理
  (cast `/Game/Ookouchi/Character/BP/BP_Player` OtherActor)
  (set `self.StartArrow` false)
  (goto _label_2))

(fn `UserConstructionScript`)
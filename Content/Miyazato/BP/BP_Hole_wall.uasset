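; BP_Hole_wall is a wall hole actor that periodically launches physics-driven rocks.
; On BeginPlay, a looping timer fires SpawnRock, which spawns a BP_Rock at an offset in the Arrow component's space.
; The rock gets physics enabled and a mass-independent velocity impulse along the Arrow's forward axis.
; The construction script adds a static mesh component stored as HoleWallEnd.
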(event `self.ReceiveBeginPlay`
  (`KismetSystemLibrary.K2_SetTimerDelegate` (delegate `SpawnRock`) 10.0 true))

(event `SpawnRock`
  (bind _returnvalue (`SceneComponent.K2_GetComponentToWorld` (`self.Arrow`)))
  (bind _returnvalue_2 (`|SpawnActorFromClass` "/Game/Miyazato/BP/BP_Rock.BP_Rock_C" (`KismetMathLibrary.MakeTransform` (`KismetMathLibrary.TransformLocation` _returnvalue (100.0 0.0 -100.0)) (.rotation _returnvalue) (.scale _returnvalue)) "Undefined" "OverrideRootScale" null null))
  (bind _rock (`/Game/Miyazato/BP/BP_Rock.Rock` _returnvalue_2))
  (`PrimitiveComponent.SetSimulatePhysics` _rock true)
  (`PrimitiveComponent.AddImpulse` _rock (`KismetMathLibrary.TransformDirection` _returnvalue (1000.0 0.0 0.0)) "None" true))

(fn `UserConstructionScript`
  (bind _returnvalue (`AddComponent|NODE_AddStaticMeshComponent-1`))
  (set `self.HoleWallEnd` _returnvalue))